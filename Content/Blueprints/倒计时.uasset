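; Countdown actor (倒计时) that shows the remaining seconds on a TextRender, then brings up the player HUDs.
; From BeginPlay, a looping one-second Delay decrements the counter and updates the text until it drops below zero.
; It then creates a HUD_me widget for MyPlayerController 0 and, if present, controller 1, reusing one HudMe variable.
; A GameState PlayerArray loop is left disconnected.
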(event EventBeginPlay
  (bind _returnvalue (Game|GetPlayerController 0))
  (bind _returnvalue_2 (Game|GetPlayerController 1))
  (Utilities|FlowControl|Delay 1.0 :!label _label)
  (bind _output_get (Variables|Default|Set倒计时时间 (- (Variables|Default|Get倒计时时间) 1)))
  (if (>= (Variables|Default|Get倒计时时间) 0)
    (Rendering|Components|TextRender|SetText (Variables|Default|GetTextRender) (Utilities|Text|ToText(Integer) _output_get))
    (goto _label)
    (else
      (Utilities|IsValid _returnvalue
        (:Is%20Valid
          (bind _asmy_player_controller (Utilities|Casting|CastToMyPlayerController _returnvalue))
          (bind _returnvalue_3 (UserInterface|CreateWidget "/Game/Blueprints/Widgets/HUD_me.HUD_me_C" _asmy_player_controller))
          (Variables|Default|Sethud_me _returnvalue_3)
          (UserInterface|Viewport|AddtoViewport (Variables|Default|Gethud_me) 0)
          (Utilities|IsValid _returnvalue_2
            (:Is%20Valid
              (bind _asmy_player_controller_2 (Utilities|Casting|CastToMyPlayerController _returnvalue_2))
              (bind _returnvalue_4 (UserInterface|CreateWidget "/Game/Blueprints/Widgets/HUD_me.HUD_me_C" _asmy_player_controller_2))
              (Variables|Default|Sethud_me _returnvalue_4)
              (UserInterface|Viewport|AddtoViewport (Variables|Default|Gethud_me) 0))))))))

(fn ConstructionScript)